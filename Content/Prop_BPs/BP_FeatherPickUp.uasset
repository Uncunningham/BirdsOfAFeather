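; BP_FeatherPickUp is a feather pickup that ends the current level when the bird player touches it.
; On first overlap it hides itself, disables bird input, plays a Wwise sound and starts a priority bird animation.
; A looping timer polls the sprite for frame 24, then fades the camera out.
; After a short delay it opens Level 2 or Level 3, chosen by the bird's Level variable.
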(event `self.Sphere.OnComponentBeginOverlap`
  (params (OverlappedComponent :type "PrimitiveComponent Object Reference") (OtherActor :type "Actor Object Reference") (OtherComp :type "PrimitiveComponent Object Reference") (OtherBodyIndex :type Integer) (bFromSweep :type Boolean) (SweepResult :type "HitResult Structure (by ref)"))
  (if (not (`self.IsTouchy?`))
    (bind _asbp_bird (cast `/Game/Character_BPs/BP_Bird` OtherActor))
    (`|ExecutionSequence`
      (:`then_0`
        (`self.SetActorHiddenInGame` true)
        (set `self.IsTouchy?` true))
      (:`then_1`
        (`self.DisableInput` _asbp_bird null))
      (:`then_2`
        (`AkGameplayStatics.PostEvent` "/Game/Wwise/Events/Play_Interact_Feather.Play_Interact_Feather" _asbp_bird))
      (:`then_4`
        (bind _asbp_bird_2 (cast `/Game/Character_BPs/BP_Bird` (`GameplayStatics.GetPlayerCharacter` 0)))
        (`/Game/Character_BPs/BP_Bird.ChangeAnimation` _asbp_bird_2 true "NewEnumerator7"))
      (:`then_5`
        (`KismetSystemLibrary.K2_SetTimerDelegate` (delegate `IsAnimOver`) 0.1 true)))))

(event `IsAnimOver`
  (bind _asbp_bird (cast `/Game/Character_BPs/BP_Bird` (`GameplayStatics.GetPlayerCharacter` 0)))
  (if (== (`PaperFlipbookComponent.GetPlaybackPositionInFrames` (`PaperCharacter.Sprite` _asbp_bird)) 24)
    (`PlayerCameraManager.StartCameraFade` :`self` (`GameplayStatics.GetPlayerCameraManager` 0) :`ToAlpha` 1.0 :`Duration` 2.0 :`bHoldWhenFinished` true)
    (`KismetSystemLibrary.Delay` 2.1)
    (if (== (`/Game/Character_BPs/BP_Bird.Level` _asbp_bird) 0)
      (`GameplayStatics.OpenLevel` "Level2_Final_V1")
      (else
        (`GameplayStatics.OpenLevel` "Level3_Final_V1")))))

(fn `UserConstructionScript`)