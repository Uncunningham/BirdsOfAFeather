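; BP_Clouds is a prop that rocks its Bugger component back and forth while something overlaps its Box.
; Begin overlap starts a looping timer that calls Shaker, and end overlap clears it.
; Shaker steps an Angle counter toward MaxAngle, adding local pitch scaled by MaxAngle each step.
; When the counter reaches MaxAngle, the sign flips, reversing the swing without Tick or a timeline.
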(event `self.Box.OnComponentBeginOverlap`
  (params (OverlappedComponent :type "PrimitiveComponent Object Reference") (OtherActor :type "Actor Object Reference") (OtherComp :type "PrimitiveComponent Object Reference") (OtherBodyIndex :type Integer) (bFromSweep :type Boolean) (SweepResult :type "HitResult Structure (by ref)"))
  (bind _returnvalue (`KismetSystemLibrary.K2_SetTimer` null "Shaker" 0.1 true)))

(event `self.Box.OnComponentEndOverlap`
  (params (OverlappedComponent :type "PrimitiveComponent Object Reference") (OtherActor :type "Actor Object Reference") (OtherComp :type "PrimitiveComponent Object Reference") (OtherBodyIndex :type Integer))
  (`KismetSystemLibrary.K2_ClearAndInvalidateTimerHandle` (stale `self.Box.OnComponentBeginOverlap` _returnvalue)))

(fn `Shaker`
  (`/Engine/EditorBlueprintResources/StandardMacros.CompareFloat` (`self.Angle`) (`self.MaxAngle`)
    (:`>`
      (set `self.Angle` (+ (`self.Angle`) -1.0))
      (`SceneComponent.K2_AddLocalRotation` (`self.Bugger`) (`KismetMathLibrary.MakeRotator` 0.0 (* 0.5 (`self.MaxAngle`))) false false :!label _label))
    (:`==`
      (set `self.MaxAngle` (* (`self.MaxAngle`) -1.0)))
    (:`<`
      (set `self.Angle` (+ (`self.Angle`) 1.0))
      (goto _label))))

(fn `UserConstructionScript`)