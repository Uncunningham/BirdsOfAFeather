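; Launch pad that springs a BP_Bird character upward after it enters the pad's box trigger.
; Overlap starts a looping timer that sinks the pad in small steps, counted by Ticker, then launches the bird at LaunchZvelo once the count reaches its threshold.
; Ending the overlap calls CheekyLand on the bird, restores the pad's starting height saved at BeginPlay, and resets the counter and timer.
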(event `self.Box.OnComponentBeginOverlap`
  (params (OverlappedComponent :type "PrimitiveComponent Object Reference") (OtherActor :type "Actor Object Reference") (OtherComp :type "PrimitiveComponent Object Reference") (OtherBodyIndex :type Integer) (bFromSweep :type Boolean) (SweepResult :type "HitResult Structure (by ref)"))
  (bind _asbp_bird (cast `/Game/Character_BPs/BP_Bird` OtherActor))
  (`KismetSystemLibrary.PrintString` "Hello")
  (bind _returnvalue (`KismetSystemLibrary.K2_SetTimerDelegate` (delegate `SpringBoard`) 0.1 true)))

(event `SpringBoard`
  (bind _returnvalue (`self.GetTransform`))
  (`self.K2_SetActorTransform` (`KismetMathLibrary.MakeTransform` (`KismetMathLibrary.MakeVector` (.x (.location _returnvalue)) (.y (.location _returnvalue)) (- (.z (.location _returnvalue)) 2.0)) (.rotation _returnvalue) (.scale _returnvalue)))
  (bind _output_get (set `self.Ticker` (+ (`self.Ticker`) 1)))
  (if (>= _output_get 12)
    (`Character.LaunchCharacter` (stale `self.Box.OnComponentBeginOverlap` _asbp_bird) (`KismetMathLibrary.MakeVector` 0.0 0.0 (`self.LaunchZvelo`)) false false)
    (`KismetSystemLibrary.K2_ClearAndInvalidateTimerHandle` (stale `self.Box.OnComponentBeginOverlap` _returnvalue))))

(event `self.ReceiveBeginPlay`
  (set `self.ReturnValueZ` (.z (.location (`self.GetTransform`)))))

(event `self.Box.OnComponentEndOverlap`
  (params (OverlappedComponent :type "PrimitiveComponent Object Reference") (OtherActor :type "Actor Object Reference") (OtherComp :type "PrimitiveComponent Object Reference") (OtherBodyIndex :type Integer))
  (bind _returnvalue (`self.GetTransform`))
  (bind _asbp_bird (cast `/Game/Character_BPs/BP_Bird` OtherActor))
  (`/Game/Character_BPs/BP_Bird.CheekyLand` _asbp_bird)
  (`self.K2_SetActorTransform` (`KismetMathLibrary.MakeTransform` (`KismetMathLibrary.MakeVector` (.x (.location _returnvalue)) (.y (.location _returnvalue)) (`self.ReturnValueZ`)) (.rotation _returnvalue) (.scale _returnvalue)))
  (set `self.Ticker` 0)
  (`KismetSystemLibrary.K2_ClearAndInvalidateTimerHandle` (stale `self.Box.OnComponentBeginOverlap` _returnvalue)))

(fn `UserConstructionScript`)