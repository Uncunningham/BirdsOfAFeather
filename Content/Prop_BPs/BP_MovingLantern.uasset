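; Moving lantern prop that travels back and forth along world X or Z and rocks while something overlaps its Box.
; Tick offsets the actor by CloudSpeed per frame, reversing when a step counter reaches PlatformRange, so motion is frame-rate dependent.
; Box overlap starts a looping Shaker timer, cleared on end overlap, that pitches the Bugger component and flips MaxAngle whenever its Angle counter reaches it.
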(event `self.Box.OnComponentBeginOverlap`
  (params (OverlappedComponent :type "PrimitiveComponent Object Reference") (OtherActor :type "Actor Object Reference") (OtherComp :type "PrimitiveComponent Object Reference") (OtherBodyIndex :type Integer) (bFromSweep :type Boolean) (SweepResult :type "HitResult Structure (by ref)"))
  (bind _returnvalue (`KismetSystemLibrary.K2_SetTimer` null "Shaker" 0.1 true)))

(event `self.Box.OnComponentEndOverlap`
  (params (OverlappedComponent :type "PrimitiveComponent Object Reference") (OtherActor :type "Actor Object Reference") (OtherComp :type "PrimitiveComponent Object Reference") (OtherBodyIndex :type Integer))
  (`KismetSystemLibrary.K2_ClearAndInvalidateTimerHandle` (stale `self.Box.OnComponentBeginOverlap` _returnvalue)))

(event `self.ReceiveTick`
  (params (DeltaSeconds :type "Float (single-precision)"))
  (bind _returnvalue (`self.GetTransform`))
  (bind _returnvalue_2 (`self.GetTransform`))
  (`/Engine/EditorBlueprintResources/StandardMacros.CompareFloat` (`self.PlatformValue`) (`self.PlatformRange`)
    (:`>`
      (set `self.PlatformValue` (+ (`self.PlatformValue`) -1.0)))
    (:`==`
      (set `self.CloudSpeed` (* (`self.CloudSpeed`) -1.0))
      (set `self.PlatformRange` (* (`self.PlatformRange`) -1.0)))
    (:`<`
      (set `self.PlatformValue` (+ (`self.PlatformValue`) 1.0))))
  (if (`self.Verticle?`)
    (`self.K2_SetActorTransform` (`KismetMathLibrary.MakeTransform` (`KismetMathLibrary.MakeVector` (.x (.location _returnvalue_2)) (.y (.location _returnvalue_2)) (+ (.z (.location _returnvalue_2)) (`self.CloudSpeed`))) (.rotation _returnvalue_2) (.scale _returnvalue_2)))
    (else
      (`self.K2_SetActorTransform` (`KismetMathLibrary.MakeTransform` (`KismetMathLibrary.MakeVector` (+ (.x (.location _returnvalue)) (`self.CloudSpeed`)) (.y (.location _returnvalue)) (.z (.location _returnvalue))) (.rotation _returnvalue) (.scale _returnvalue))))))

(fn `Shaker`
  (`/Engine/EditorBlueprintResources/StandardMacros.CompareFloat` (`self.Angle`) (`self.MaxAngle`)
    (:`>`
      (set `self.Angle` (+ (`self.Angle`) -1.0))
      (`SceneComponent.K2_AddLocalRotation` (`self.Bugger`) (`KismetMathLibrary.MakeRotator` 0.0 (* 0.5 (`self.MaxAngle`))) false false :!label _label))
    (:`==`
      (set `self.MaxAngle` (* (`self.MaxAngle`) -1.0)))
    (:`<`
      (set `self.Angle` (+ (`self.Angle`) 1.0))
      (goto _label))))

(fn `UserConstructionScript`)