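; BP_Gale is a wind-zone prop that pushes the player's BP_Bird while it is inside the trigger Box.
; Box overlap begin and end events for a BP_Bird toggle a Push flag.
; While Push is set, Tick moves player character 0 by Force along world Z or X, chosen by the Vertical flag, using SetActorTransform.
; The offset is applied per frame without delta-time scaling.
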(event `self.Box.OnComponentBeginOverlap`
  (params (OverlappedComponent :type "PrimitiveComponent Object Reference") (OtherActor :type "Actor Object Reference") (OtherComp :type "PrimitiveComponent Object Reference") (OtherBodyIndex :type Integer) (bFromSweep :type Boolean) (SweepResult :type "HitResult Structure (by ref)"))
  (cast `/Game/Character_BPs/BP_Bird` OtherActor)
  (set `self.Push?` true))

(event `self.Box.OnComponentEndOverlap`
  (params (OverlappedComponent :type "PrimitiveComponent Object Reference") (OtherActor :type "Actor Object Reference") (OtherComp :type "PrimitiveComponent Object Reference") (OtherBodyIndex :type Integer))
  (cast `/Game/Character_BPs/BP_Bird` OtherActor)
  (set `self.Push?` false))

(event `self.ReceiveTick`
  (params (DeltaSeconds :type "Float (single-precision)"))
  (bind _force (`self.Force`))
  (if (`self.Push?`)
    (bind _asbp_bird (cast `/Game/Character_BPs/BP_Bird` (`GameplayStatics.GetPlayerCharacter` 0)))
    (if (`self.Vertical`)
      (bind _returnvalue (`self.GetTransform` _asbp_bird))
      (`self.K2_SetActorTransform` _asbp_bird (`KismetMathLibrary.MakeTransform` (`KismetMathLibrary.MakeVector` (.x (.location _returnvalue)) (.y (.location _returnvalue)) (+ (.z (.location _returnvalue)) _force)) (.rotation _returnvalue) (.scale _returnvalue)) false false)
      (else
        (`self.K2_SetActorTransform` _asbp_bird (`KismetMathLibrary.MakeTransform` (`KismetMathLibrary.MakeVector` (+ (.x (.location _returnvalue)) _force) (.y (.location _returnvalue)) (.z (.location _returnvalue))) (.rotation _returnvalue) (.scale _returnvalue)) false false)))))

(fn `UserConstructionScript`)