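; BP_DistanceLight is a light prop that changes its point light's intensity based on the player character's position.
; Each tick it takes the signed X-axis offset between the light and the player, subtracts it from MaxIntensity, and applies the result to the light.
; MaxIntensity is overwritten each time, so the change accumulates across frames.
; The offset is also printed on screen for debugging.
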(event `self.ReceiveTick`
  (params (DeltaSeconds :type "Float (single-precision)"))
  (bind _returnvalue_x (`KismetMathLibrary.BreakVector` (`SceneComponent.K2_GetComponentLocation` (`self.PointLight`))))
  (bind _returnvalue_x_2 (`KismetMathLibrary.BreakVector` (`self.K2_GetActorLocation` (`GameplayStatics.GetPlayerCharacter` 0))))
  (bind _output_get (set `self.Distance` (- _returnvalue_x _returnvalue_x_2)))
  (bind _output_get_2 (set `self.MaxIntensity` (- (`self.MaxIntensity`) _output_get)))
  (`KismetSystemLibrary.PrintString` (`KismetStringLibrary.Conv_DoubleToString` _output_get) true true (struct :`G` 0.66 :`B` 1.0 :`A` 1.0) 0.01)
  (`LightComponent.SetIntensity` (`self.PointLight`) _output_get_2))

(fn `UserConstructionScript`)