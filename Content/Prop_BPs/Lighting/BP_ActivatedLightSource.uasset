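; BP_ActivatedLightSource is a light prop that brightens its PointLight when something begins overlapping its Sphere trigger.
; The overlap sets a Switch flag, and the Light function, called every Tick, raises intensity by a fixed, frame-rate-dependent step until it passes DesiredIntensity, then clears the flag.
; Nothing dims the light again, and debug prints fire on overlap and on each step.
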(event `self.ReceiveTick`
  (params (DeltaSeconds :type "Float (single-precision)"))
  (`self.Light`))

(event `self.Sphere.OnComponentBeginOverlap`
  (params (OverlappedComponent :type "PrimitiveComponent Object Reference") (OtherActor :type "Actor Object Reference") (OtherComp :type "PrimitiveComponent Object Reference") (OtherBodyIndex :type Integer) (bFromSweep :type Boolean) (SweepResult :type "HitResult Structure (by ref)"))
  (`KismetSystemLibrary.PrintString` "Hello")
  (set `self.Switch` true))

(fn `Light`
  (if (and (`self.Switch`) (<= (`self.CurrentIntensity`) (`self.DesiredIntensity`)))
    (bind _output_get (set `self.CurrentIntensity` (+ (`self.CurrentIntensity`) 100.0)))
    (`KismetSystemLibrary.PrintString` (`KismetStringLibrary.Conv_DoubleToString` _output_get) true true (struct :`G` 0.66 :`B` 1.0 :`A` 1.0) 0.01)
    (`LightComponent.SetIntensity` (`self.PointLight`) _output_get)
    (else
      (set `self.Switch` false))))

(fn `UserConstructionScript`)