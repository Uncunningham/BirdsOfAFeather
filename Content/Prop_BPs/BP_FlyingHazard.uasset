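; Flying hazard prop that patrols back and forth and penalizes any BP_Bird overlapping its box by calling GotHit and emptying its GlideMeter.
; Each Tick steps a counter by one toward HazardRange, flipping both range and speed when they are equal.
; The Verticle flag selects world Z or X movement by HazardSpeed, applied per frame without delta time.
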(event `self.Box.OnComponentBeginOverlap`
  (params (OverlappedComponent :type "PrimitiveComponent Object Reference") (OtherActor :type "Actor Object Reference") (OtherComp :type "PrimitiveComponent Object Reference") (OtherBodyIndex :type Integer) (bFromSweep :type Boolean) (SweepResult :type "HitResult Structure (by ref)"))
  (bind _asbp_bird (cast `/Game/Character_BPs/BP_Bird` OtherActor))
  (`/Game/Character_BPs/BP_Bird.GotHit` _asbp_bird)
  (set `/Game/Character_BPs/BP_Bird.GlideMeter` 0.0 _asbp_bird))

(event `self.ReceiveTick`
  (params (DeltaSeconds :type "Float (single-precision)"))
  (bind _returnvalue (`self.GetTransform`))
  (bind _returnvalue_2 (`self.GetTransform`))
  (`/Engine/EditorBlueprintResources/StandardMacros.CompareFloat` (`self.HazardValue`) (`self.HazardRange`)
    (:`>`
      (set `self.HazardValue` (+ (`self.HazardValue`) -1.0)))
    (:`==`
      (set `self.HazardSpeed` (* (`self.HazardSpeed`) -1.0))
      (set `self.HazardRange` (* (`self.HazardRange`) -1.0)))
    (:`<`
      (set `self.HazardValue` (+ (`self.HazardValue`) 1.0))))
  (if (`self.Verticle?`)
    (`self.K2_SetActorTransform` (`KismetMathLibrary.MakeTransform` (`KismetMathLibrary.MakeVector` (.x (.location _returnvalue_2)) (.y (.location _returnvalue_2)) (+ (.z (.location _returnvalue_2)) (`self.HazardSpeed`))) (.rotation _returnvalue_2) (.scale _returnvalue_2)))
    (else
      (`self.K2_SetActorTransform` (`KismetMathLibrary.MakeTransform` (`KismetMathLibrary.MakeVector` (+ (.x (.location _returnvalue)) (`self.HazardSpeed`)) (.y (.location _returnvalue)) (.z (.location _returnvalue))) (.rotation _returnvalue) (.scale _returnvalue))))))

(fn `UserConstructionScript`)